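; BP_Hero is a hero character for FallingSurvive that can deploy a parachute while falling.
; Pressing F mid-fall passes a DoOnce gate, spawns and attaches BP_Parachute, sharply cuts velocity, nearly removes gravity and raises air control.
; Pressing T or landing destroys the parachute, restores movement settings and resets the gate for the next deployment.
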(event EventBeginPlay
  (|CallParentFunction) ; This node is disabled and will not be called.\nDrag off pins to build functionality.
)

(event Collision|EventActorBeginOverlap
  (params (OtherActor :type Actor%20Object%20Reference))
  (|CallParentFunction OtherActor) ; This node is disabled and will not be called.\nDrag off pins to build functionality.
)

(event EventTick
  (params (DeltaSeconds :type Float%20%28single-precision%29))
  (|CallParentFunction DeltaSeconds) ; This node is disabled and will not be called.\nDrag off pins to build functionality.
)

(event EventOnLanded
  (params (Hit :type Hit%20Result%20Structure%20%28by%20ref%29))
  (bind _charactermovement (Variables|Character|GetCharacterMovement))
  (bind _charactermovement_2 (Variables|Character|GetCharacterMovement))
  (Actor|DestroyActor (stale Input|KeyboardEvents|F _returnvalue))
  (Variables|/Script/Engine.CharacterMovementComponent|SetAirControl _charactermovement_2 0.2)
  (Variables|/Script/Engine.CharacterMovementComponent|SetGravityScale _charactermovement_2 1.0)
  (Utilities|FlowControl|DoOnce false) ; enters at Reset
)

(event Input|KeyboardEvents|F
  (params (Key :type Key%20Structure :default "None"))
  (bind _charactermovement (Variables|Character|GetCharacterMovement))
  (:Pressed
    (if (AI|Components|NavMovement|IsFalling (Variables|Character|GetCharacterMovement))
      (Utilities|FlowControl|DoOnce false
        (:Completed
          (bind _returnvalue (Game|SpawnActorfromClass "/Game/FallingSurvive/Staff/Equipment/Parachute/BP_Parachute.BP_Parachute_C" (Transformation|GetWorldTransform (Variables|Default|GetScene)) "Undefined" 0 0))
          (Transformation|AttachActorToActor _returnvalue (Game|GetPlayerCharacter 0) "None" "KeepWorld" "KeepWorld" "KeepWorld" true)
          (Variables|/Script/Engine.MovementComponent|SetVelocity _charactermovement (Math|Vector|Lerp(Vector) "0, 0, 0" (Transformation|GetVelocity) 0.1))
          (Variables|/Script/Engine.CharacterMovementComponent|SetAirControl _charactermovement 0.3)
          (Variables|/Script/Engine.CharacterMovementComponent|SetGravityScale _charactermovement 0.01))))))

(event Input|KeyboardEvents|T
  (params (Key :type Key%20Structure :default "None"))
  (bind _charactermovement (Variables|Character|GetCharacterMovement))
  (bind _charactermovement_2 (Variables|Character|GetCharacterMovement))
  (:Pressed
    (Actor|DestroyActor (stale Input|KeyboardEvents|F _returnvalue))
    (Variables|/Script/Engine.CharacterMovementComponent|SetAirControl _charactermovement_2 0.2)
    (Variables|/Script/Engine.CharacterMovementComponent|SetGravityScale _charactermovement_2 1.0)
    (Utilities|FlowControl|DoOnce false) ; enters at Reset
  ))

(fn ConstructionScript
  (|CallParentFunction))